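; Player character for a 2D side-scrolling game that runs, jumps via key or touch, collects coins and dies on touching an enemy.
; A State enum drives flipbook animation through a Select, and movement along X flips control yaw to face the direction.
; Death disables input, calls OnDeath and sends updated game data with the best coin score to the GameInstance's save dispatcher.
; The achievement update is a pass-through stub.
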(event Custom|Death
  ;[1 1 1] On Death
  (Variables|Default|SetState "NewEnumerator3")
  (Input|DisableInput (Game|GetPlayerController 0))
  (CallFunction|StateChange)
  (Default|CallOnDeath)
  (bind _gamedata (CallFunction|UpdateGameData))
  (bind _asglobal_game_instance (Utilities|Casting|CastToGlobalGameInstance (Game|GetGameInstance)))
  (Default|CallSaveGameDispatcher _asglobal_game_instance _gamedata))

(event Custom|StateChange
  ;[1 1 1] Handle Animation
  (bind _newparam (CallFunction|AnimationStateMachine (Variables|Default|GetState)))
  (Sprite|SetFlipbook (Variables|Default|GetSprite) _newparam))

(event EventBeginPlay
  ;[1 1 1] Multiplayer
  (Class|ActorComponent|SetIsReplicated (Variables|Default|GetSprite) true)
  ;[1 1 1] Load Game Data
  (bind _asglobal_game_instance (Utilities|Casting|CastToGlobalGameInstance (Game|GetGameInstance)))
  (Variables|Default|SetCurrentGame (Variables|/Game/Blueprints/GameElements/GlobalGameInstance.GlobalGameInstance_C|GetGameData _asglobal_game_instance)))

(event EventOnLanded
  (params (Hit :type Hit%20Result%20Structure%20%28by%20ref%29))
  ;[1 1 1] Handle Landed
  (bind _isdead (CallFunction|IsDead))
  (if (not _isdead)
    (Variables|Default|SetState "NewEnumerator0")
    (CallFunction|StateChange)))

(event Collision|EventActorBeginOverlap
  (params (OtherActor :type Actor%20Object%20Reference))
  ;[1 1 1] Hit Check
  (if (Utilities|ClassIsChildOf (Utilities|GetClass OtherActor) "/Game/Blueprints/GameElements/Enemy.Enemy_C")
    (bind _isdead (CallFunction|IsDead))
    (if (not _isdead)
      (CallFunction|Death))
    (elif (Utilities|ClassIsChildOf (Utilities|GetClass OtherActor) "/Game/Blueprints/GameElements/Coin.Coin_C")
      (bind _isdead_2 (CallFunction|IsDead))
      (if (not _isdead_2)
        (Math|Integer|IncrementInt (Variables|Default|GetCoinsCollected))))))

(event Input|ActionEvents|InputActionJump
  ;[1 1 1] Handle Jump
  (:Pressed
    (Character|Jump)
    (Variables|Default|SetState "NewEnumerator2")
    (CallFunction|StateChange))
  (:Released
    (Character|StopJumping)))

(event Input|AxisEvents|InputAxisMoveRight
  (params (AxisValue :type Float%20%28single-precision%29))
  ;[1 1 1] Handle movement
  (Pawn|Input|AddMovementInput "1.000000, 0, 0" AxisValue false)
  (Math|Float|CompareFloat AxisValue 0.0
    (:>
      (Pawn|SetControlRotation (Pawn|GetController) (Class|KismetMathLibrary|MakeRot 0.0 0.0 0.0))
      (Variables|Default|SetState "NewEnumerator1" :!label _label)
      (CallFunction|StateChange))
    (:==
      (Variables|Default|SetState "NewEnumerator0")
      (CallFunction|StateChange))
    (:<
      (Pawn|SetControlRotation (Pawn|GetController) (Class|KismetMathLibrary|MakeRot 0.0 1.8e+02 0.0))
      (goto _label))))

(event Input|TouchEvents|InputTouch
  (params (Location :type Vector) (FingerIndex :type ETouchIndex%20Enum))
  ;[1 1 1] Handle Jump
  (:Pressed
    (Character|Jump)
    (Variables|Default|SetState "NewEnumerator2")
    (CallFunction|StateChange))
  (:Released
    (Character|StopJumping)))

(fn ConstructionScript)

(fn AnimationStateMachine
  (params (CharacterState :type CharacterState%20Enum))
  (return (Utilities|Select :Index CharacterState :NewEnumerator0 (Variables|Flipbooks|GetIdle) :NewEnumerator1 (Variables|Flipbooks|GetRunning) :NewEnumerator2 (Variables|Flipbooks|GetJumping) :NewEnumerator3 (Variables|Flipbooks|GetDead))))

(fn IsDead
  (return (Utilities|Enum|Equal(Enum) (Variables|Default|GetState) "NewEnumerator3")))

(fn UpdateGameData
  (bind _currentgame (Variables|Default|GetCurrentGame))
  (bind (_numberofgames _bestscore _maxtime _achivements) (Utilities|Struct|BreakPersistentData _currentgame))
  (bind _achivements_out (CallFunction|UpdateAchivements _achivements))
  (return (Utilities|Struct|MakePersistentData (stale _result) (Math|Integer|Max(Integer) _bestscore (Variables|Default|GetCoinsCollected)) _maxtime _achivements_out)))

(fn UpdateAchivements
  (params (Achivements%20In :type Array%20of%20Booleans))
  (return Achivements%20In))