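; Game instance that holds persistent player data and syncs it with platform leaderboard and achievements.
; Init loads or creates the save object, then queries the CoinScore leaderboard and caches achievements.
; A save dispatcher event updates the in-memory data and reruns both syncs, but SaveGameData is never called.
; Leaderboard sync adopts the remote score unless the local best is higher, when it writes zero; achievement sync is an empty stub.
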(event Custom|SaveGameDispatcherEvent
  (params (CurrentGame :type Persistent%20Data%20Structure))
  (Utilities|FlowControl|Sequence
    (:then_0
      ;[1 1 1] Update Data
      (Variables|Default|SetGameData CurrentGame))
    (:then_1
      ;[1 1 1] Sync With Remote Leaderboard
      (bind _leaderboardvalue (|LeaderboardQuery (Game|GetPlayerController 0) "CoinScore")
        (:OnSuccess
          (CallFunction|SyncLeaderboard (Variables|Default|GetGameData) _leaderboardvalue))))
    (:then_2
      ;[1 1 1] Sync With Remote Achivements
      (|CacheAchievements (Game|GetPlayerController 0)
        (:OnSuccess
          (CallFunction|SyncAchivements (Variables|Default|GetGameData)))))))

(event EventInit
  (Utilities|FlowControl|Sequence
    (:then_0
      ;[1 1 1] InitializeGameData
      (EventDispatchers|BindEventtoSaveGameDispatcher (delegate Custom|SaveGameDispatcherEvent))
      (bind _returnvalue (SaveGame|DoesSaveGameExist "Save"))
      (if _returnvalue
        (CallFunction|LoadGameData)
        (else
          (CallFunction|CreateGameData))))
    (:then_1
      ;[1 1 1] Sync With Remote Leaderboard
      (bind _leaderboardvalue (|LeaderboardQuery (Game|GetPlayerController 0) "CoinScore")
        (:OnSuccess
          (CallFunction|SyncLeaderboard (Variables|Default|GetGameData) _leaderboardvalue))))
    (:then_2
      ;[1 1 1] Sync With Remote Achivements
      (|CacheAchievements (Game|GetPlayerController 0)
        (:OnSuccess
          (CallFunction|SyncAchivements (Variables|Default|GetGameData)))))))

(fn CreateGameData
  (bind _returnvalue (SaveGame|CreateSaveGameObject "/Game/Blueprints/GameElements/GameData.GameData_C"))
  (Variables|Default|SetSaveGame _returnvalue))

(fn LoadGameData
  (bind _returnvalue (SaveGame|LoadGamefromSlot "Save"))
  (bind _output_get (Variables|Default|SetSaveGame _returnvalue))
  (bind _asgame_data (Utilities|Casting|CastToGameData _output_get))
  (Variables|Default|SetGameData (Utilities|Struct|MakePersistentData (.NumberOfGames (Utilities|Struct|BreakPersistentData (Variables|/Game/Blueprints/GameElements/GameData.GameData_C|GetPersistentData _asgame_data))) (.BestScore (Utilities|Struct|BreakPersistentData (Variables|/Game/Blueprints/GameElements/GameData.GameData_C|GetPersistentData _asgame_data))) (.MaxTime (Utilities|Struct|BreakPersistentData (Variables|/Game/Blueprints/GameElements/GameData.GameData_C|GetPersistentData _asgame_data))) (.Achivements (Utilities|Struct|BreakPersistentData (Variables|/Game/Blueprints/GameElements/GameData.GameData_C|GetPersistentData _asgame_data))))))

(fn SaveGameData
  (params (GameData :type Persistent%20Data%20Structure))
  (bind (_numberofgames _bestscore _maxtime _achivements) (Utilities|Struct|BreakPersistentData GameData))
  (bind _asgame_data (Utilities|Casting|CastToGameData (Variables|Default|GetSaveGame)))
  (Variables|/Game/Blueprints/GameElements/GameData.GameData_C|SetPersistentData _asgame_data (Utilities|Struct|MakePersistentData _numberofgames _bestscore _maxtime _achivements))
  (SaveGame|SaveGametoSlot _asgame_data "Save"))

(fn SyncLeaderboard
  (params (PersistentData :type Persistent%20Data%20Structure%20%28by%20ref%29) (HighScore :type Integer))
  (bind (_numberofgames _bestscore _maxtime _achivements) (Utilities|Struct|BreakPersistentData PersistentData))
  (if (< HighScore _bestscore)
    (Class|LeaderboardBlueprintLibrary|WriteLeaderboardInteger (Game|GetPlayerController 0) "CoinScore")
    (else
      (Variables|Default|SetGameData (Utilities|Struct|MakePersistentData _numberofgames HighScore _maxtime _achivements))))
  (return))

(fn SyncAchivements
  (params (Data :type Persistent%20Data%20Structure)))